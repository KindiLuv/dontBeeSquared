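; BP_Pawn is a player camera pawn that pans, zooms and rotates in 45-degree steps.
; Input events update desired location, rotation and spring arm length, with movement following the actor's forward and right vectors and zoom clamped to a range.
; Tick interpolates the actor transform and arm length toward those targets for smooth motion, without sweeping for collision.
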(event `self.ReceiveBeginPlay`
  (set `self.Location_Desired` (`self.K2_GetActorLocation`))
  (set `self.ZoomDesired` (`SpringArmComponent.TargetArmLength` (`self.SpringArm`)))
  (set `self.Rotation_Desired` (`self.K2_GetActorRotation`)))

(event `self.ReceiveTick`
  (params (DeltaSeconds :type "Float (single-precision)"))
  (bind _springarm (`self.SpringArm`))
  (set `SpringArmComponent.TargetArmLength` (`KismetMathLibrary.FInterpTo` (`SpringArmComponent.TargetArmLength` _springarm) (`self.ZoomDesired`) DeltaSeconds 2.0) _springarm)
  (`self.K2_SetActorLocation` (`KismetMathLibrary.VInterpTo` (`self.K2_GetActorLocation`) (`self.Location_Desired`) DeltaSeconds 5.0))
  (`self.K2_SetActorRotation` (`KismetMathLibrary.RInterpTo` (`self.K2_GetActorRotation`) (`self.Rotation_Desired`) DeltaSeconds 5.0)))

(event `InputAxis|InputAxis_Zoom`
  (params (AxisValue :type "Float (single-precision)"))
  (set `self.ZoomDesired` (`KismetMathLibrary.FClamp` (+ (`self.ZoomDesired`) (* AxisValue 100.0)) 100.0 5000.0)))

(event `InputAxis|InputAxis_Forward`
  (params (AxisValue :type "Float (single-precision)"))
  (set `self.Location_Desired` (+ (`self.Location_Desired`) (* (* AxisValue 100.0) (`self.GetActorForwardVector`)))))

(event `InputAxis|InputAxis_Right`
  (params (AxisValue :type "Float (single-precision)"))
  (set `self.Location_Desired` (+ (`self.Location_Desired`) (* (* AxisValue 100.0) (`self.GetActorRightVector`)))))

(event `InputAction|InputAction_RotationRight`
  (params (Key :type "Key Structure"))
  (:`Pressed`
    (set `self.Rotation_Desired` (`KismetMathLibrary.ComposeRotators` (`self.Rotation_Desired`) (struct :`Yaw` -45.0)))))

(event `InputAction|InputAction_RotationLeft`
  (params (Key :type "Key Structure"))
  (:`Pressed`
    (set `self.Rotation_Desired` (`KismetMathLibrary.ComposeRotators` (`self.Rotation_Desired`) (struct :`Yaw` 45.0)))))

(fn `UserConstructionScript`)